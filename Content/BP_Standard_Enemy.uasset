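; BP_Standard_Enemy is an enemy that moves along the world X axis and dies when shot.
; On BeginPlay it stores its starting position, and a Timeline track offsets it from that point with a swept move.
; When the Timeline finishes, it calls Play again after a short delay.
; A hit from BP_FirstPersonProjectile destroys both the projectile and the enemy.
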(event Collision|EventHit
  (params (MyComp :type Primitive%20Component%20Object%20Reference) (Other :type Actor%20Object%20Reference) (OtherComp :type Primitive%20Component%20Object%20Reference) (bSelfMoved :type Boolean) (HitLocation :type Vector :default "0, 0, 0") (HitNormal :type Vector :default "0, 0, 0") (NormalImpulse :type Vector :default "0, 0, 0") (Hit :type Hit%20Result%20Structure%20%28by%20ref%29))
  (bind _asbp_first_person_projectile (Utilities|Casting|CastToBP_FirstPersonProjectile Other))
  (Actor|DestroyActor _asbp_first_person_projectile)
  (Actor|DestroyActor))

(event EventBeginPlay
  (Variables|Default|SetStarting%20Postion (Transformation|GetActorLocation))
  (bind _newtrack_0 (Timeline|Timeline PlayFromStart)
    (:Update
      (Transformation|SetActorLocation (+ (Variables|Default|GetStarting%20Postion) (Math|Vector|MakeVector _newtrack_0 0.0 0.0)) true false))
    (:Finished
      (Utilities|FlowControl|Delay 0.1)
      (Timeline|Timeline Play))))

(fn ConstructionScript)